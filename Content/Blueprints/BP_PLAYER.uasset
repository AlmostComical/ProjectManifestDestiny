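; Player character for a 2D flipbook side-scroller, with walking, jumping and an attack.
; Enhanced Input drives movement along world X and turns control rotation to face the travel direction.
; Each tick, UpdateAnim picks an idle, walk, jump or fall flipbook from ground state and velocity.
; Attack input only plays an override sequence on the anim instance, with no hit logic here.
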(event Input|EnhancedActionEvents|EnhancedInputActionIA_JUMP
  (params (ActionValue :type Boolean) (ElapsedSeconds :type Float%20%28double-precision%29) (TriggeredSeconds :type Float%20%28double-precision%29) (InputAction :type Input%20Action%20Object%20Reference :default "/Game/Input/Actions/IA_JUMP.IA_JUMP"))
  (:Started
    (Character|Jump))
  (:Completed
    (Character|StopJumping)))

(event Input|EnhancedActionEvents|EnhancedInputActionIA_MOVE
  (params (ActionValue :type Float%20%28double-precision%29) (ElapsedSeconds :type Float%20%28double-precision%29) (TriggeredSeconds :type Float%20%28double-precision%29) (InputAction :type Input%20Action%20Object%20Reference :default "/Game/Input/Actions/IA_MOVE.IA_MOVE"))
  (Pawn|Input|AddMovementInput "1.000000,0.000000,0.000000" ActionValue false)
  (Pawn|SetControlRotation (Pawn|GetController) (select (> ActionValue 0.0) (Math|Rotator|MakeRotator 0.0 0.0 1.8e+02) (Math|Rotator|MakeRotator 0.0 0.0 0.0))))

(event Input|EnhancedActionEvents|EnhancedInputActionIA_ATTACK
  (params (ActionValue :type Float%20%28double-precision%29) (ElapsedSeconds :type Float%20%28double-precision%29) (TriggeredSeconds :type Float%20%28double-precision%29) (InputAction :type Input%20Action%20Object%20Reference :default "/Game/Input/Actions/IA_ATTACK.IA_ATTACK"))
  (:Started
    (|PlayAnimationOverridewithCallbacks (Class|PaperZDCharacter|GetAnimInstance) "/Game/Blueprints/AnimSequences/ATTACK.ATTACK" "DefaultSlot" 1.0 0.0)))

(event EventBeginPlay
  (|CallParentFunction)
  (bind _asplayer_controller (Utilities|Casting|CastToPlayerController (Pawn|GetController)))
  (Input|AddMappingContext (PlayerController|LocalPlayerSubsystems|GetEnhancedInputLocalPlayerSubsystem _asplayer_controller) "/Game/Input/Actions/IMC_PLATFORMING.IMC_PLATFORMING" 0 "(bIgnoreAllPressedKeysUntilRelease=True,bForceImmediately=False,bNotifyUserSettings=False)"))

(event EventTick
  (params (DeltaSeconds :type Float%20%28single-precision%29))
  (|CallParentFunction 0.0)
  (CallFunction|UpdateAnim (Variables|Default|GetSprite)))

(fn ConstructionScript)

(fn UpdateAnim
  (params (self2 :type Paper%20Flipbook%20Component%20Object%20Reference))
  (if (AI|Components|NavMovement|IsMovingonGround (Variables|Character|GetCharacterMovement))
    (if (> (Math|Vector|VectorLength (Transformation|GetVelocity)) 0.0)
      (Sprite|SetFlipbook (Variables|Default|GetSprite) "/Game/PaperAssets/Characters/Flipbooks/FP_PLAYER_WALK.FP_PLAYER_WALK")
      (else
        (Sprite|SetFlipbook self2 "/Game/PaperAssets/Characters/Flipbooks/FP_PLAYER_IDLE.FP_PLAYER_IDLE")))
    (elif (< (.z (Transformation|GetVelocity)) -1e+02)
      (Sprite|SetFlipbook (Variables|Default|GetSprite) "/Game/PaperAssets/Characters/Flipbooks/FP_PLAYER_FALL.FP_PLAYER_FALL")
      (else
        (Sprite|SetFlipbook (Variables|Default|GetSprite) "/Game/PaperAssets/Characters/Flipbooks/FP_PLAYER_JUMP.FP_PLAYER_JUMP")))))